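; Dog enemy that chases the player, leaps at them and deals damage on capsule contact.
; Pawn sensing triggers an AI MoveTo chase that leads into a cooldown-limited launch, gated by a stagger flag stored on the player.
; Incoming damage drains armor before health, reveals a health bar widget and destroys the dog at zero health.
; Capsule overlap with direct line of sight registers the dog as the player's kick target.
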(event OnComponentBeginOverlap(CapsuleComponent)
  (params (OverlappedComponent :type Primitive%20Component%20Object%20Reference) (OtherActor :type Actor%20Object%20Reference) (OtherComp :type Primitive%20Component%20Object%20Reference) (OtherBodyIndex :type Integer) (bFromSweep :type Boolean) (SweepResult :type Hit%20Result%20Structure%20%28by%20ref%29))
  ;[1 1 1] In Range for Kick
  (if (== OtherActor (Variables|Default|GetPlayer))
    (if (Variables|Default|GetDirectSightPlayer)
      (if true
        (Variables|/Game/Razor_Character/Razor_BP.Razor_BP_C|SetCan%20Kick (Variables|Default|GetPlayer) true)
        (if (not (Utilities|IsValid (Variables|/Game/Razor_Character/Razor_BP.Razor_BP_C|GetKickable%20Character (Variables|Default|GetPlayer))))
          (Variables|/Game/Razor_Character/Razor_BP.Razor_BP_C|SetKickable%20Character (Variables|Default|GetPlayer) self))))))

(event OnComponentEndOverlap(CapsuleComponent)
  (params (OverlappedComponent :type Primitive%20Component%20Object%20Reference) (OtherActor :type Actor%20Object%20Reference) (OtherComp :type Primitive%20Component%20Object%20Reference) (OtherBodyIndex :type Integer))
  (bind (_asrazor_bp _bsuccess) (Utilities|Casting|CastToRazor_BP OtherActor))
  ;[1 1 1] Out of Kick Range
  (if _bsuccess
    (Variables|/Game/Razor_Character/Razor_BP.Razor_BP_C|SetCan%20Kick _asrazor_bp false)
    (Variables|/Game/Razor_Character/Razor_BP.Razor_BP_C|SetKickable%20Character _asrazor_bp 0)))

(event OnComponentHit(CapsuleComponent)
  (params (HitComponent :type Primitive%20Component%20Object%20Reference) (OtherActor :type Actor%20Object%20Reference) (OtherComp :type Primitive%20Component%20Object%20Reference) (NormalImpulse :type Vector :default "0, 0, 0") (Hit :type Hit%20Result%20Structure%20%28by%20ref%29))
  ;[1 1 1] Deal Damage to Player
  (if (== OtherActor (Variables|Default|GetPlayer))
    (Utilities|FlowControl|DoOnce false :!label _label
      (:Completed
        (Game|Damage|ApplyDamage (Variables|Default|GetPlayer) 4e+01 0 0 "/Script/Engine.DamageType")
        (Components|Movement|StopMovementImmediately (Variables|Character|GetCharacterMovement))))
    (else
      (Utilities|FlowControl|Delay 1.0)
      (goto _label Reset))))

(event Custom|Jump%20at%20Player
  ;[1 1 1] Jump At Player
  (Utilities|FlowControl|DoOnce false
    (:Completed
      (Utilities|FlowControl|Delay 0.25)
      (Utilities|IfStaggered
        (:else
          (Character|LaunchCharacter (|GetLaunchVelocity) true false)
          (CallFunction|ResetJump))))))

(event Custom|Reset%20Jump
  ;[1 1 1] Jump At Player
  (Utilities|FlowControl|Delay 2.0)
  (Utilities|FlowControl|DoOnce false) ; enters at Reset
)

(event EventTick
  (params (DeltaSeconds :type Float%20%28single-precision%29))
  ;[1 1 1] Chase Player
  (Utilities|IfStaggered
    (:else
      (if (Variables|Default|GetSees%20Player)
        (|TracePlayer)
        (AI|AIMoveTo self "0, 0, 0" (Variables|Default|GetPlayer) 5e+02 true
          (:OnSuccess
            (Utilities|IfStaggered
              (:else
                (CallFunction|JumpatPlayer))))
          (:OnFail
            (CallFunction|ResetJump)))))))

(event Game|Damage|EventAnyDamage
  (params (Damage :type Float%20%28single-precision%29) (DamageType :type Damage%20Type%20Object%20Reference) (InstigatedBy :type Controller%20Object%20Reference) (DamageCauser :type Actor%20Object%20Reference))
  (bind _health (Variables|Default|GetHealth))
  ;[1 1 1] Take Damage
  (CallFunction|TakeDamage Damage)
  (Rendering|SetVisibility (Variables|Default|GetHealth%20Bar) true false)
  (|SetHealthBar _health (Variables|Default|GetArmor))
  (if (<= _health 0.0)
    (Actor|DestroyActor)))

(fn ConstructionScript)

(fn TakeDamage
  (params (Damage :type Float%20%28single-precision%29))
  (bind _returnvalue (/ Damage 1e+02))
  (if (> (Variables|Default|GetArmor) 0.0)
    (Variables|Default|SetArmor (- (Variables|Default|GetArmor) _returnvalue))
    (else
      (Variables|Default|SetHealth (- (Variables|Default|GetHealth) _returnvalue)))))

(event OnSeePawn(PawnSensing)
  (params (Pawn :type Pawn%20Object%20Reference))
  (bind _player (Variables|Default|GetPlayer))
  (bind _returnvalue (== Pawn _player))
  ;[1 1 1] See the player
  (if _returnvalue
    _
    (else
      _))
  (Variables|Default|SetSees%20Player _returnvalue))

(event OnHearNoise(PawnSensing)
  (params (Instigator :type Pawn%20Object%20Reference) (Location :type Vector%20%28by%20ref%29 :default "0, 0, 0") (Volume :type Float%20%28single-precision%29))
  (bind _player (Variables|Default|GetPlayer))
  (bind _returnvalue (== Instigator _player))
  ;[1 1 1] Hear the player
  (if _returnvalue
    _
    (else
      _))
  (Variables|Default|SetSees%20Player _returnvalue))

(event EventBeginPlay
  (Variables|Default|SetEnemy%20Health%20Bar (.AsDoggie%20Health (Utilities|Casting|CastToDoggie_Health (UserInterface|GetUserWidgetObject (Variables|Default|GetHealth%20Bar)))))
  (Variables|Default|SetPlayer (.AsRazor%20BP (Utilities|Casting|CastToRazor_BP (Game|Player|GetPlayerPawn 0))))
  (return))